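; BP_Spline_Road is a road Blueprint that builds a procedural mesh from spline points in its construction script.
; It appends each point's local position to Vertices, then creates one mesh section using grid triangle indices.
; The grid uses the point count for both dimensions, so its indices expect N×N vertices while the loop adds only N.
; AddProceduralMesh is an empty stub, and the event graph has no logic.
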(event EventBeginPlay)

(event Collision|EventActorBeginOverlap
  (params (OtherActor :type Actor%20Object%20Reference)))

(event EventTick
  (params (DeltaSeconds :type Float%20%28single-precision%29)))

(fn ConstructionScript
  (bind _spline (Variables|Default|GetSpline))
  (bind _returnvalue (Spline|GetNumberOfSplinePoints _spline))
  (for _index (range 0 (- _returnvalue 1))
    (Utilities|Array|Add (Variables|Default|GetVertices) (Spline|GetLocationatSplinePoint (Variables|Default|GetSpline) _index "Local")))
  (bind _triangles (Class|KismetProceduralMeshLibrary|CreateGridMeshTriangles _returnvalue _returnvalue false))
  (Class|ProceduralMeshComponent|CreateMeshSectionLinearColor (Variables|Default|GetProdualMesh) 0 (Variables|Default|GetVertices) _triangles 0 0 0 0 0 0 0 false))

(fn AddProceduralMesh
  (params (NewParam :type Boolean) (NewParam1 :type Boolean) (NewParam2 :type Boolean) (NewParam3 :type Boolean)))