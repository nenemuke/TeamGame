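; Human gunner enemy, a child Blueprint that sets its combat status, nurture status and reward data on BeginPlay before calling the parent.
; Its SpecialAttack override triggers the Fire event, which waits briefly, then calls PlayMontage on the mesh.
; Fire also spawns rifle muzzle flash and sound at the weapon socket, plus a Bullet_Human at the AttackArrow transform that receives the enemy's AttackPower.
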(event Custom|Fire
  (bind _weapon (Variables|Default|GetWeapon))
  (bind _returnvalue (Transformation|GetSocketTransform _weapon "MuzzleFlash" "RTS_World"))
  (Utilities|FlowControl|Delay 0.2)
  (Animation|Montage|PlayMontage (Variables|Character|GetMesh) 0
    (:then
      (Effects|SpawnEmitteratLocation "/Game/MilitaryWeapDark/FX/P_AssaultRifle_MuzzleFlash.P_AssaultRifle_MuzzleFlash" (.location _returnvalue) (.rotation _returnvalue))
      (Audio|PlaySoundatLocation "/Game/MilitaryWeapDark/Sound/Rifle/RifleB_Fire_Cue.RifleB_Fire_Cue" (.location _returnvalue) "0, 0, 0" 1.0 1.0 0.0 0 0 0 0)
      (bind _returnvalue_2 (Game|SpawnActorfromClass "/Game/Assets/Blueprints/Human/GunHuman/Bullet_Human.Bullet_Human_C" (Transformation|GetWorldTransform (Variables|Default|GetAttackArrow)) "Undefined" 0 0))
      (Default|SetSpecialAttackPower _returnvalue_2 (Variables|Default|GetAttackPower)))))

(event EventBeginPlay
  (Variables|Default|SetStatus (Utilities|Struct|MakeAnimalAIStatus 2.5e+03 2e+02 0.0 0.0 0 0.0 0.0 "/Game/FlexibleCombatSystem/Montages/M_Fists_AttackA.M_Fists_AttackA" 0.0 5.0 5e+01 2e+02 1e+02 3e+02 "/Game/FlexibleCombatSystem/Animations/Common/HitImpact_Montage.HitImpact_Montage" 3.0 0.0))
  (Variables|Default|SetNurtureStatus (Utilities|Struct|MakeNurtureStatus 0.0 0.0 0.0 0.0 0.0 0.0 0.0 7e+01 3e+01 0.0 5e+01 3e+01 0.0 0.0 7e+01 0.0 0.0))
  (Variables|Default|SetHumanReward (Utilities|Struct|MakeHumanReward 8 1500 1))
  (|CallParentFunction))

(event Collision|EventActorBeginOverlap
  (params (OtherActor :type Actor%20Object%20Reference))
  (|CallParentFunction OtherActor) ; このノードは無効になっているため呼び出せません。\n機能をビルドするにはピンをドラッグしてください。
)

(event EventTick
  (params (DeltaSeconds :type Float%20%28single-precision%29))
  (|CallParentFunction DeltaSeconds) ; このノードは無効になっているため呼び出せません。\n機能をビルドするにはピンをドラッグしてください。
)

(fn ConstructionScript
  (|CallParentFunction))

(fn SpecialAttack
  (CallFunction|Fire))