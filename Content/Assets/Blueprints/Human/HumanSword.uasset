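; HumanSword is the sword variant of a human unit, defined as a data-only style child of a parent Blueprint.
; On BeginPlay it fills the inherited Status, NurtureStatus and HumanReward structs and the attack animation speed, then calls the parent BeginPlay.
; Its attack and hit montages are set inside Status, with the attack using an axe-and-shield animation.
; All other behavior comes from the parent, as Tick and overlap events are disabled stubs.
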(event EventBeginPlay
  (Variables|Default|SetStatus (Utilities|Struct|MakeAnimalAIStatus 1e+01 1.0 0.0 0.0 0 0.0 0.0 "/Game/FlexibleCombatSystem/Montages/M_AxeAndShield_AttackA.M_AxeAndShield_AttackA" 0.0 5.0 5e+01 8e+02 1e+02 3e+02 "/Game/FlexibleCombatSystem/Animations/Common/HitImpact_Montage.HitImpact_Montage" 1e+02))
  (Variables|Default|SetNurtureStatus (Utilities|Struct|MakeNurtureStatus 1e+03 0.0 0.0 0.0 0.0 0.0 0.0 5e+01 5e+01 0.0 5e+01 1e+02 0.0 0.0 3e+01 0.0 0.0))
  (Variables|Default|SetHumanReward (Utilities|Struct|MakeHumanReward 10 10 1))
  (Variables|Default|SetAttackAnimeSpeed 2.5)
  (|CallParentFunction))

(event Collision|EventActorBeginOverlap
  (params (OtherActor :type Actor%20Object%20Reference))
  (|CallParentFunction OtherActor) ; このノードは無効になっているため呼び出せません。\n機能をビルドするにはピンをドラッグしてください。
)

(event EventTick
  (params (DeltaSeconds :type Float%20%28single-precision%29))
  (|CallParentFunction DeltaSeconds) ; このノードは無効になっているため呼び出せません。\n機能をビルドするにはピンをドラッグしてください。
)

(fn ConstructionScript
  (|CallParentFunction))