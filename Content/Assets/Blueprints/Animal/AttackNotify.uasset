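; Animation notify state that marks the attack window in animal and AI attack animations.
; On begin and end, it casts the mesh owner to Animal_BP, falling back to AIBP, and calls that actor's AttackStart or AttackEnd.
; Other owner types are ignored.
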(fn ReceivedNotifyBegin
  (params (MeshComp :type Skeletal%20Mesh%20Component%20Object%20Reference) (Animation :type Anim%20Sequence%20Base%20Object%20Reference) (TotalDuration :type Float%20%28single-precision%29) (EventReference :type Anim%20Notify%20Event%20Reference%20Structure%20%28by%20ref%29))
  (bind _returnvalue (Components|GetOwner MeshComp))
  (bind _asanimal_bp (Utilities|Casting|CastToAnimal_BP _returnvalue)
    (:then
      (Default|AttackStart _asanimal_bp))
    (:CastFailed
      (bind _asaibp (Utilities|Casting|CastToAIBP _returnvalue))
      (Default|AttackStart _asaibp)))
  (return false))

(fn ReceivedNotifyEnd
  (params (MeshComp :type Skeletal%20Mesh%20Component%20Object%20Reference) (Animation :type Anim%20Sequence%20Base%20Object%20Reference) (EventReference :type Anim%20Notify%20Event%20Reference%20Structure%20%28by%20ref%29))
  (bind _returnvalue (Components|GetOwner MeshComp))
  (bind _asanimal_bp (Utilities|Casting|CastToAnimal_BP _returnvalue)
    (:then
      (Default|AttackEnd _asanimal_bp))
    (:CastFailed
      (bind _asaibp (Utilities|Casting|CastToAIBP _returnvalue))
      (Default|AttackEnd _asaibp)))
  (return false))