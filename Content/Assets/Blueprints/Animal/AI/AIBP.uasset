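; Base AI character for animal and human combatants, covering stats, combat, death and UI (name tag in the Zoo level, HP bar elsewhere).
; Stats combine Status and NurtureStatus, with nurture values also rolling back-move and player-chase behavior.
; Overlap volumes detect enemies, bait and the player, feeding flags and Blackboard keys alongside damage reactions and target distance.
; IsAnimal selects opponents, montage attacks deduplicate hits, and death ragdolls the mesh.
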(event EventTick
  (params (DeltaSeconds :type Float%20%28single-precision%29))
  (|ＨＰバーの処理)
  (|残りＨＰ計算)
  (|ターゲットアクターとの距離を計算)
  (if (Variables|Default|GetIsDeath)
    (|死んだら判定無くす)))

(event Collision|EventActorBeginOverlap
  (params (OtherActor :type Actor%20Object%20Reference)))

(event EventBeginPlay
  (|初期化))

(fn ConstructionScript)

(fn SetName
  (bind _name (Variables|Default|GetName))
  (bind _hp (Variables|Default|GetHP))
  (bind _returnvalue (Game|GetCurrentLevelName true))
  (if (Utilities|Enum|Equal(Enum) _returnvalue "Zoo")
    (bind _returnvalue_2 (UserInterface|CreateWidget "/Game/Assets/Blueprints/Animal/WBP_Name.WBP_Name_C" 0 _name))
    (bind _output_get (Variables|Default|SetNameBar _returnvalue_2))
    (UserInterface|Viewport|AddtoViewport _output_get 0)
    (else
      (bind _returnvalue_3 (UserInterface|CreateWidget "/Game/Assets/Blueprints/Animal/WBP_HPBar.WBP_HPBar_C" 0 _name _hp _hp))
      (bind _output_get_2 (Variables|Default|SetHPBar _returnvalue_3))
      (UserInterface|Viewport|AddtoViewport _output_get_2 0)
      (Variables|/Game/Assets/Blueprints/Animal/WBP_HPBar.WBP_HPBar_C|SetMainHP _output_get_2 (Variables|Default|GetHP)))))

(fn AttackStart
  (Collision|SetCollisionEnabled (Variables|Default|GetDamageCollision) "QueryAndPhysics"))

(fn AttackEnd
  (Collision|SetCollisionEnabled (Variables|Default|GetDamageCollision) "NoCollision")
  (Utilities|Array|Clear (Variables|Default|GetAttackActor)))

(fn Rest
  (Variables|Default|SetIsRest true))

(fn FinishRest
  (Variables|Default|SetIsRest false))

(fn Alert
  (Variables|Default|SetIsAlert true))

(fn FinishAlert
  (Variables|Default|SetIsAlert false))

(fn KeepDistance
  (Variables|Default|SetIsKeepDistance true))

(fn FinishKeepDistance
  (Variables|Default|SetIsKeepDistance false))

(fn ChangeWalkSpeed
  (Variables|/Script/Engine.CharacterMovementComponent|SetMaxWalkSpeed (Variables|Character|GetCharacterMovement) (Variables|Default|GetWalkSpeed)))

(fn ChangeRunSpeed
  (Variables|/Script/Engine.CharacterMovementComponent|SetMaxWalkSpeed (Variables|Character|GetCharacterMovement) (Variables|Default|GetRunSpeed)))

(fn ChangeKeepDistanceSpeed
  (Variables|/Script/Engine.CharacterMovementComponent|SetMaxWalkSpeed (Variables|Character|GetCharacterMovement) (Variables|Default|GetKeepDistanceSpeed)))

(fn EscapeActorSet
  (bind _lastattackedactor (Variables|Default|GetLastAttackedActor))
  (bind _asaibp (Utilities|Casting|CastToAIBP _lastattackedactor)
    (:then
      (if (<= (Variables|AIBP_C|GetHP _asaibp) 0.0)
        (AI|Components|Blackboard|SetValueasObject (AI|GetBlackboard 0) (Utilities|Name|MakeLiteralName "EscapeActor") 0 :!label _label)
        (else
          (AI|Components|Blackboard|SetValueasObject (AI|GetBlackboard 0) (Utilities|Name|MakeLiteralName "EscapeActor") (Variables|Default|GetLastAttackedActor) :!label _label_2))))
    (:CastFailed
      (bind _asanimal_bp (Utilities|Casting|CastToAnimal_BP _lastattackedactor))
      (if (<= (Variables|/Game/Assets/Blueprints/Animal/Animal_BP.Animal_BP_C|GetHP _asanimal_bp) 0.0)
        (goto _label)
        (else
          (goto _label_2))))))

(fn ChangeAnimalHPBar
  (bind _hp (Variables|Default|GetHP))
  (if (<= _hp 0.0)
    (CallFunction|Death)
    (Widget|RemovefromParent (Variables|Default|GetHPBar))
    (else
      (Default|HPSet (Variables|Default|GetHPBar) _hp))))

(fn DestroyUI
  (Widget|RemovefromParent (Variables|Default|GetHPBar)))

(fn SpecialAttack
  (Game|SpawnActorfromClass "/Game/Assets/Blueprints/Animal/Fox/Bullet_Fox.Bullet_Fox_C" (Transformation|GetWorldTransform (Variables|Default|GetAttackArrow)) "Undefined" 0 0))

(event OnComponentEndOverlap(BaitCollision)
  (params (OverlappedComponent :type Primitive%20Component%20Object%20Reference) (OtherActor :type Actor%20Object%20Reference) (OtherComp :type Primitive%20Component%20Object%20Reference) (OtherBodyIndex :type Integer))
  (bind _baitarray (Variables|Default|GetBaitArray))
  (bind _asbait (Utilities|Casting|CastToBait OtherActor)
    (:then
      (Utilities|Array|RemoveIndex _baitarray (Utilities|Array|FindItem _baitarray _asbait)))
    (:CastFailed
      (Utilities|Casting|CastToClichanBP_2 OtherActor)
      (AI|Components|Blackboard|SetValueasObject (AI|GetBlackboard 0) (Utilities|Name|MakeLiteralName "PlayerClose") 0)
      (Variables|Default|SetIsPlayerChase false))))

(event Game|Damage|EventAnyDamage
  (params (Damage :type Float%20%28single-precision%29) (DamageType :type Damage%20Type%20Object%20Reference) (InstigatedBy :type Controller%20Object%20Reference) (DamageCauser :type Actor%20Object%20Reference))
  (Variables|Default|SetHP (- (Variables|Default|GetHP) Damage))
  (Default|OnTakeDamage (Variables|Default|GetHPBar) Damage)
  (if (<= (Variables|Default|GetHP) 0.0)
    (CallFunction|Death)
    (Utilities|FlowControl|Delay 2.0)
    (Widget|RemovefromParent (Variables|Default|GetHPBar))
    (else
      (AI|Components|Blackboard|SetValueasObject (AI|GetBlackboard 0) (Utilities|Name|MakeLiteralName "TargetActor") DamageCauser)
      (AI|Components|Blackboard|SetValueasBool (AI|GetBlackboard 0) (Utilities|Name|MakeLiteralName "IsDamaged") true)
      (Variables|Default|SetLastAttackedActor DamageCauser)
      (CallFunction|EscapeActorSet))))

(event Custom|Attack
  (if (not (Variables|Default|GetIsAttack))
    (Animation|Montage|PlayMontage (Variables|Character|GetMesh) (Variables|Default|GetAttack%20Montage)
      (:then
        (Variables|Default|SetIsAttack true))
      (:OnCompleted
        (Variables|Default|SetIsAttack false)))))

(event OnComponentBeginOverlap(TouchCollision)
  (params (OverlappedComponent :type Primitive%20Component%20Object%20Reference) (OtherActor :type Actor%20Object%20Reference) (OtherComp :type Primitive%20Component%20Object%20Reference) (OtherBodyIndex :type Integer) (bFromSweep :type Boolean) (SweepResult :type Hit%20Result%20Structure%20%28by%20ref%29))
  (if (Variables|Default|GetIsAnimal)
    (bind _ashuman_aibp (Utilities|Casting|CastToHumanAIBP OtherActor)
      (:then
        (if (== (Variables|AIBP_C|GetBodyCollision _ashuman_aibp) OtherComp)
          (if (> (Variables|AIBP_C|GetHP _ashuman_aibp) 0.0)
            (Variables|Default|SetIsTouch true)
            (else
              (Variables|Default|SetIsTouch false)))))
      (:CastFailed
        (Utilities|Casting|CastToBait OtherActor
          (:then
            (AI|Components|Blackboard|SetValueasBool (AI|GetBlackboard 0) (Utilities|Name|MakeLiteralName "IsBaitTouch") true))
          (:CastFailed
            (if (Variables|Default|GetIsPlayerChase)
              (Utilities|Casting|CastToClichanBP_2 OtherActor)
              (AI|Components|Blackboard|SetValueasBool (AI|GetBlackboard 0) (Utilities|Name|MakeLiteralName "IsPlayerTouch") true))))))
    (else
      (bind _asanimal_aibp (Utilities|Casting|CastToAnimalAIBP OtherActor)
        (:then
          (if (== (Variables|AIBP_C|GetBodyCollision _asanimal_aibp) OtherComp)
            (if (> (Variables|AIBP_C|GetHP _asanimal_aibp) 0.0)
              (Variables|Default|SetIsTouch true)
              (else
                (Variables|Default|SetIsTouch false)))))
        (:CastFailed
          (bind _asanimal_bp (Utilities|Casting|CastToAnimal_BP OtherActor))
          (if (== (Variables|/Game/Assets/Blueprints/Animal/Animal_BP.Animal_BP_C|GetBox _asanimal_bp) OtherComp)
            (if (> (Variables|/Game/Assets/Blueprints/Animal/Animal_BP.Animal_BP_C|GetHP _asanimal_bp) 0.0)
              (Variables|Default|SetIsTouch true)
              (else
                (Variables|Default|SetIsTouch false)))))))))

(event OnComponentEndOverlap(TouchCollision)
  (params (OverlappedComponent :type Primitive%20Component%20Object%20Reference) (OtherActor :type Actor%20Object%20Reference) (OtherComp :type Primitive%20Component%20Object%20Reference) (OtherBodyIndex :type Integer))
  (if (Variables|Default|GetIsAnimal)
    (bind _ashuman_aibp (Utilities|Casting|CastToHumanAIBP OtherActor)
      (:then
        (if (== (Variables|AIBP_C|GetBodyCollision _ashuman_aibp) OtherComp)
          (Variables|Default|SetIsTouch false)))
      (:CastFailed
        (Utilities|Casting|CastToBait OtherActor
          (:then
            (AI|Components|Blackboard|SetValueasBool (AI|GetBlackboard 0) (Utilities|Name|MakeLiteralName "IsBaitTouch") false))
          (:CastFailed
            (if (Variables|Default|GetIsPlayerChase)
              (Utilities|Casting|CastToClichanBP_2 OtherActor)
              (AI|Components|Blackboard|SetValueasBool (AI|GetBlackboard 0) (Utilities|Name|MakeLiteralName "IsPlayerTouch") false))))))
    (else
      (bind _asanimal_bp (Utilities|Casting|CastToAnimal_BP OtherActor)
        (:then
          (if (== (Variables|/Game/Assets/Blueprints/Animal/Animal_BP.Animal_BP_C|GetBox _asanimal_bp) OtherComp)
            (Variables|Default|SetIsTouch false)))
        (:CastFailed
          (bind _asanimal_aibp (Utilities|Casting|CastToAnimalAIBP OtherActor))
          (if (== (Variables|AIBP_C|GetBodyCollision _asanimal_aibp) OtherComp)
            (Variables|Default|SetIsTouch false)))))))

(event OnComponentBeginOverlap(EnemyCollision)
  (params (OverlappedComponent :type Primitive%20Component%20Object%20Reference) (OtherActor :type Actor%20Object%20Reference) (OtherComp :type Primitive%20Component%20Object%20Reference) (OtherBodyIndex :type Integer) (bFromSweep :type Boolean) (SweepResult :type Hit%20Result%20Structure%20%28by%20ref%29))
  (if (Variables|Default|GetIsAnimal)
    (bind _ashuman_aibp (Utilities|Casting|CastToHumanAIBP OtherActor))
    (if (== (Variables|AIBP_C|GetBodyCollision _ashuman_aibp) OtherComp)
      (Variables|Default|SetIsEnemyClose true))
    (else
      (bind _asanimal_bp (Utilities|Casting|CastToAnimal_BP OtherActor)
        (:then
          (if (== (Variables|/Game/Assets/Blueprints/Animal/Animal_BP.Animal_BP_C|GetBox _asanimal_bp) OtherComp)
            (Variables|Default|SetIsEnemyClose true :!label _label)))
        (:CastFailed
          (bind _asanimal_aibp (Utilities|Casting|CastToAnimalAIBP OtherActor))
          (if (== (Variables|AIBP_C|GetBodyCollision _asanimal_aibp) OtherComp)
            (goto _label)))))))

(event OnComponentEndOverlap(EnemyCollision)
  (params (OverlappedComponent :type Primitive%20Component%20Object%20Reference) (OtherActor :type Actor%20Object%20Reference) (OtherComp :type Primitive%20Component%20Object%20Reference) (OtherBodyIndex :type Integer))
  (if (Variables|Default|GetIsAnimal)
    (bind _ashuman_aibp (Utilities|Casting|CastToHumanAIBP OtherActor))
    (if (== (Variables|AIBP_C|GetBodyCollision _ashuman_aibp) OtherComp)
      (Variables|Default|SetIsEnemyClose false))
    (else
      (bind _asanimal_bp (Utilities|Casting|CastToAnimal_BP OtherActor)
        (:then
          (if (== (Variables|/Game/Assets/Blueprints/Animal/Animal_BP.Animal_BP_C|GetBox _asanimal_bp) OtherComp)
            (Variables|Default|SetIsEnemyClose false :!label _label)))
        (:CastFailed
          (bind _asanimal_aibp (Utilities|Casting|CastToAnimalAIBP OtherActor))
          (if (== (Variables|AIBP_C|GetBodyCollision _asanimal_aibp) OtherComp)
            (goto _label)))))))

(event OnComponentBeginOverlap(DamageCollision)
  (params (OverlappedComponent :type Primitive%20Component%20Object%20Reference) (OtherActor :type Actor%20Object%20Reference) (OtherComp :type Primitive%20Component%20Object%20Reference) (OtherBodyIndex :type Integer) (bFromSweep :type Boolean) (SweepResult :type Hit%20Result%20Structure%20%28by%20ref%29))
  (if (not (Variables|Default|GetIsDeath))
    (if (Variables|Default|GetIsAnimal)
      ;[1 1 1] 人のＡＩにダメージを与える
      (bind _ashuman_aibp (Utilities|Casting|CastToHumanAIBP OtherActor))
      (if (not (Utilities|Array|ContainsItem (Variables|Default|GetAttackActor) (Utilities|GetDisplayName _ashuman_aibp)))
        (if (== (Variables|AIBP_C|GetBodyCollision _ashuman_aibp) OtherComp)
          (Game|Damage|ApplyDamage OtherActor (Variables|Default|GetAttackPower) 0 self)
          (Utilities|Array|Add (Variables|Default|GetAttackActor) (Utilities|GetDisplayName _ashuman_aibp))))
      (else
        ;[1 1 1] 動物ＡＩにダメージを与える
        (bind _asanimal_aibp (Utilities|Casting|CastToAnimalAIBP OtherActor)
          (:then
            (if (not (Utilities|Array|ContainsItem (Variables|Default|GetAttackActor) (Utilities|GetDisplayName _asanimal_aibp)))
              (if (== (Variables|AIBP_C|GetBodyCollision _asanimal_aibp) OtherComp)
                (Game|Damage|ApplyDamage OtherActor (Variables|Default|GetAttackPower) 0 self)
                (Utilities|Array|Add (Variables|Default|GetAttackActor) (Utilities|GetDisplayName _asanimal_aibp)))))
          (:CastFailed
            ;[1 1 1] プレイヤーにダメージを与える
            (bind _asanimal_bp (Utilities|Casting|CastToAnimal_BP OtherActor))
            (if (not (Utilities|Array|ContainsItem (Variables|Default|GetAttackActor) (Utilities|GetDisplayName _asanimal_bp)))
              (if (== (Variables|/Game/Assets/Blueprints/Animal/Animal_BP.Animal_BP_C|GetBox _asanimal_bp) OtherComp)
                (Game|Damage|ApplyDamage OtherActor (Variables|Default|GetAttackPower) 0 self)
                (Utilities|Array|Add (Variables|Default|GetAttackActor) (Utilities|GetDisplayName _asanimal_bp))))))))))

(event Custom|Death
  (if (not (Variables|Default|GetIsDeath))
    (Physics|SetSimulatePhysics (Variables|Character|GetMesh) true)
    (Collision|SetCollisionEnabled (Variables|Default|GetBodyCollision) "NoCollision")
    (Variables|Default|SetIsDeath true)))

(event OnComponentBeginOverlap(BaitCollision)
  (params (OverlappedComponent :type Primitive%20Component%20Object%20Reference) (OtherActor :type Actor%20Object%20Reference) (OtherComp :type Primitive%20Component%20Object%20Reference) (OtherBodyIndex :type Integer) (bFromSweep :type Boolean) (SweepResult :type Hit%20Result%20Structure%20%28by%20ref%29))
  (bind _asbait (Utilities|Casting|CastToBait OtherActor)
    (:then
      (if (== (Utilities|Array|FindItem (Variables|Default|GetBaitArray) _asbait) -1)
        (Utilities|Array|Add (Variables|Default|GetBaitArray) _asbait)))
    (:CastFailed
      (if (<= (Math|Random|RandomFloatinRange 0.0 1e+02) (.PlayerChase (Utilities|Struct|BreakNurtureStatus (Variables|Default|GetNurtureStatus))))
        (Utilities|Casting|CastToClichanBP_2 OtherActor)
        (AI|Components|Blackboard|SetValueasObject (AI|GetBlackboard 0) (Utilities|Name|MakeLiteralName "PlayerClose") (Game|Player|GetPlayerPawn 0))
        (Variables|Default|SetIsPlayerChase true)))))