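; Quest system Blueprint that builds the stage for the quest selected by QuestNum and returns its PlayerStart and ClearTime.
; StartQuest reads the quest's data table row, spawns the stage base, then spawns parts placed by stage table rows.
; EnemySpawnPosition components on those parts supply a location array, which each enemy indexes by FirstPosition when spawned.
; Before enemies spawn, the player pawn is teleported to the row's PlayerSetAnimalCamera location.
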(event EventBeginPlay)

(event Collision|EventActorBeginOverlap
  (params (OtherActor :type Actor%20Object%20Reference)))

(event EventTick
  (params (DeltaSeconds :type Float%20%28single-precision%29)))

(fn ConstructionScript)

(fn StartQuest
  (Variables|Default|SetPlayerPawn 0)
  (bind _returnvalue (Utilities|GetDataTableRow "/Game/Assets/Blueprints/Quest/QuestDaTatable.QuestDaTatable" (Utilities|String|StringToName (Utilities|String|ToString(Integer) (Variables|Default|GetQuestNum))))
    (:then
      (Variables|Default|SetQuestInfo _returnvalue)
      (|ステージのベース生成)
      (|ステージのパーツ生成
        (:Completed
          (|プレイヤーの座標設定)
          (|敵の生成
            (:Completed
              (return (.PlayerStart (Utilities|Struct|BreakQuestInfo (Variables|Default|GetQuestInfo))) (.ClearTime (Utilities|Struct|BreakQuestInfo (Variables|Default|GetQuestInfo)))))))))))