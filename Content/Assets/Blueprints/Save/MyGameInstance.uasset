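; Game instance that persists animal-raising and player data (money, action points, food, truck level) in two SaveGame slots.
; Each mutator reloads its slot, edits the data and saves immediately, with animals matched by name.
; New animals randomly split ten points across five stats, each point worth one percent of that species' DataTable maximum.
; A text-input widget, checked through a polling function, supplies the animal's name.
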(fn LoadAnimalNurture
  (bind _returnvalue (SaveGame|LoadGamefromSlot "AnimalStatus"))
  (Utilities|IsValid _returnvalue
    (:Is%20Valid
      (bind _assave_animal_nurture (Utilities|Casting|CastToSaveAnimalNurture _returnvalue))
      (Variables|Default|SetAnimalStatusData _assave_animal_nurture))
    (:Is%20Not%20Valid
      (bind _returnvalue_2 (SaveGame|CreateSaveGameObject "/Game/Assets/Blueprints/Save/SaveAnimalNurture.SaveAnimalNurture_C"))
      (Variables|Default|SetAnimalStatusData _returnvalue_2))))

(fn SaveAnimalNurture
  (SaveGame|SaveGametoSlot (Variables|Default|GetAnimalStatusData) "AnimalStatus"))

(fn AddAnimalNurture
  (params (NewItem :type Nurture%20Data%20Structure%20%28by%20ref%29))
  (Utilities|Array|Add (Variables|/Game/Assets/Blueprints/Save/SaveAnimalNurture.SaveAnimalNurture_C|GetAnimalNurtureData (Variables|Default|GetAnimalStatusData)) NewItem))

(fn ResetAnimalNurture
  (CallFunction|LoadAnimalNurture)
  (Utilities|Array|Clear (Variables|/Game/Assets/Blueprints/Save/SaveAnimalNurture.SaveAnimalNurture_C|GetAnimalNurtureData (Variables|Default|GetAnimalStatusData)))
  (CallFunction|SaveAnimalNurture))

(fn SaveNewAnimal
  (params (ClassName :type String))
  (CallFunction|LoadAnimalNurture)
  (|初期ステータスをランダムで決定 ClassName)
  (CallFunction|AddAnimalNurture (Utilities|Struct|MakeNurtureData (Variables|Default|GetName) ClassName (Variables|Default|GetMaxNurtureStatus) 1))
  (CallFunction|SaveAnimalNurture))

(fn NurtureDataUpdate
  (params (Name :type String) (NurtureData :type Nurture%20Data%20Structure%20%28by%20ref%29) (Item%20Status :type Nurture%20Status%20Structure))
  (bind (_name _classname _status _level _experience) (Utilities|Struct|BreakNurtureData NurtureData))
  (bind _animalstatusdata (Variables|Default|GetAnimalStatusData))
  (bind _animalnurturedata (Variables|/Game/Assets/Blueprints/Save/SaveAnimalNurture.SaveAnimalNurture_C|GetAnimalNurtureData _animalstatusdata))
  (CallFunction|LoadAnimalNurture)
  (for (_array_element _array_index) _animalnurturedata
    (if (Utilities|Enum|Equal(Enum) (.Name (Utilities|Struct|BreakNurtureData _array_element)) Name)
      (Utilities|Array|SetArrayElem _animalnurturedata _array_index (Utilities|Struct|MakeNurtureData (.Name (Utilities|Struct|BreakNurtureData _array_element)) (.ClassName (Utilities|Struct|BreakNurtureData _array_element)) Item%20Status _level _experience))
      (CallFunction|SaveAnimalNurture))))

(fn StatusUpdate
  (params (Name :type String) (Item%20Status :type Nurture%20Status%20Structure))
  (bind _animalstatusdata (Variables|Default|GetAnimalStatusData))
  (bind _animalnurturedata (Variables|/Game/Assets/Blueprints/Save/SaveAnimalNurture.SaveAnimalNurture_C|GetAnimalNurtureData _animalstatusdata))
  (CallFunction|LoadAnimalNurture)
  (for (_array_element _array_index) _animalnurturedata
    (if (Utilities|Enum|Equal(Enum) (.Name (Utilities|Struct|BreakNurtureData _array_element)) Name)
      (Utilities|Array|SetArrayElem _animalnurturedata _array_index (Utilities|Struct|MakeNurtureData (.Name (Utilities|Struct|BreakNurtureData _array_element)) (.ClassName (Utilities|Struct|BreakNurtureData _array_element)) Item%20Status (.Level (Utilities|Struct|BreakNurtureData _array_element)) (.Experience (Utilities|Struct|BreakNurtureData _array_element))))
      (CallFunction|SaveAnimalNurture))))

(fn InputName
  (bind _returnvalue (UserInterface|CreateWidget "/Game/Assets/UI/Base/WB_TextInput_Base.WB_TextInput_Base_C"))
  (bind _output_get (Variables|Default|SetTextInput _returnvalue))
  (UserInterface|Viewport|AddtoViewport _output_get 0)
  (Default|SetAllNurture _output_get (Variables|Default|GetAnimalStatusData)))

(fn TickCheckNameFinish
  (bind _textinput (Variables|Default|GetTextInput)
    (:then
      (bind _animalname (Default|GetAnimalName _textinput))
      (Variables|Default|SetName _animalname)
      (return (Variables|/Game/Assets/UI/Base/WB_TextInput_Base.WB_TextInput_Base_C|GetIsFinishInput _textinput)))
    (:else
      (return false))))

(fn DeleteAnimal
  (params (B :type String))
  (bind _animalstatusdata (Variables|Default|GetAnimalStatusData))
  (bind _animalnurturedata (Variables|/Game/Assets/Blueprints/Save/SaveAnimalNurture.SaveAnimalNurture_C|GetAnimalNurtureData _animalstatusdata))
  (CallFunction|LoadAnimalNurture)
  (for (_array_element _array_index) _animalnurturedata
    (if (Utilities|Enum|Equal(Enum) (.Name (Utilities|Struct|BreakNurtureData _array_element)) B)
      (Utilities|Array|RemoveIndex _animalnurturedata _array_index)
      (CallFunction|SaveAnimalNurture))))

(fn LoadPlayerData
  (bind _returnvalue (SaveGame|LoadGamefromSlot "PlayerData"))
  (Utilities|IsValid _returnvalue
    (:Is%20Valid
      (bind _assave_player_data (Utilities|Casting|CastToSavePlayerData _returnvalue))
      (Variables|Default|SetPlayerData _assave_player_data))
    (:Is%20Not%20Valid
      (bind _returnvalue_2 (SaveGame|CreateSaveGameObject "/Game/Assets/Blueprints/Save/SavePlayerData.SavePlayerData_C"))
      (Variables|Default|SetPlayerData _returnvalue_2))))

(fn SavePlayerData
  (SaveGame|SaveGametoSlot (Variables|Default|GetPlayerData) "PlayerData"))

(fn GetMoney
  (params (Money :type Integer))
  (bind _playerdata (Variables|Default|GetPlayerData))
  (CallFunction|LoadPlayerData)
  (Variables|/Game/Assets/Blueprints/Save/SavePlayerData.SavePlayerData_C|SetMoney _playerdata (+ (Variables|/Game/Assets/Blueprints/Save/SavePlayerData.SavePlayerData_C|GetMoney _playerdata) Money))
  (CallFunction|SavePlayerData))

(fn GetActionPoint
  (params (ActionPoint :type Integer))
  (bind _playerdata (Variables|Default|GetPlayerData))
  (CallFunction|LoadPlayerData)
  (Variables|/Game/Assets/Blueprints/Save/SavePlayerData.SavePlayerData_C|SetActionPoint _playerdata (+ (Variables|/Game/Assets/Blueprints/Save/SavePlayerData.SavePlayerData_C|GetActionPoint _playerdata) ActionPoint))
  (CallFunction|SavePlayerData))

(fn AddAppleNum
  (params (AppleNum :type Integer))
  (bind _playerdata (Variables|Default|GetPlayerData))
  (CallFunction|LoadPlayerData)
  (Variables|/Game/Assets/Blueprints/Save/SavePlayerData.SavePlayerData_C|SetAppleNum _playerdata (+ (Variables|/Game/Assets/Blueprints/Save/SavePlayerData.SavePlayerData_C|GetAppleNum _playerdata) AppleNum))
  (CallFunction|SavePlayerData))

(fn AddGrassNum
  (params (GrassNum :type Integer))
  (bind _playerdata (Variables|Default|GetPlayerData))
  (CallFunction|LoadPlayerData)
  (Variables|/Game/Assets/Blueprints/Save/SavePlayerData.SavePlayerData_C|SetGrassNum _playerdata (+ (Variables|/Game/Assets/Blueprints/Save/SavePlayerData.SavePlayerData_C|GetGrassNum _playerdata) GrassNum))
  (CallFunction|SavePlayerData))

(fn AddMeatNum
  (params (MeatNum :type Integer))
  (bind _playerdata (Variables|Default|GetPlayerData))
  (CallFunction|LoadPlayerData)
  (Variables|/Game/Assets/Blueprints/Save/SavePlayerData.SavePlayerData_C|SetMeatNum _playerdata (+ (Variables|/Game/Assets/Blueprints/Save/SavePlayerData.SavePlayerData_C|GetMeatNum _playerdata) MeatNum))
  (CallFunction|SavePlayerData))

(fn AddTruckLevel
  (params (TruckLevel :type Integer))
  (bind _playerdata (Variables|Default|GetPlayerData))
  (CallFunction|LoadPlayerData)
  (Variables|/Game/Assets/Blueprints/Save/SavePlayerData.SavePlayerData_C|SetTruckLevel _playerdata (+ (Variables|/Game/Assets/Blueprints/Save/SavePlayerData.SavePlayerData_C|GetTruckLevel _playerdata) TruckLevel))
  (CallFunction|SavePlayerData))