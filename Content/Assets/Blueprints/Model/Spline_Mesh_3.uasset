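; Spline mesh placement actor that lays out a set number of static mesh components along its spline in the construction script.
; Meshes are evenly spaced from start to end, using world spline locations converted to actor-local space.
; OrientToSpline gives every mesh the rotation sampled at the spline's start, rather than at its own distance.
; An Instanced Static Mesh version with per-point rotation is left disconnected, and the event graph is empty.
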(event EventBeginPlay)

(event Collision|EventActorBeginOverlap
  (params (OtherActor :type Actor%20Object%20Reference)))

(event EventTick
  (params (DeltaSeconds :type Float%20%28single-precision%29)))

(fn ConstructionScript
  (bind _numberofmeshs (Variables|Default|GetNumberOfMeshs))
  (bind _returnvalue (- _numberofmeshs 1))
  (if (> _numberofmeshs 0)
    (for _index (range 0 _returnvalue)
      (bind _returnvalue_2 (AddComponent|AddStaticMeshComponent false (Math|Conversions|ToTransform(Vector) (Math|Transform|InverseTransformLocation (Transformation|GetActorTransform) (Spline|GetLocationatDistanceAlongSpline (Variables|Default|GetSpline) (* _index (/ (Spline|GetSplineLength (Variables|Default|GetSpline)) (Math|Conversions|ToFloat(Integer) _returnvalue))) "World")))))
      (if (Variables|Default|GetOrientToSpline)
        (Transformation|SetWorldRotation _returnvalue_2 (Spline|GetRotationatDistanceAlongSpline (Variables|Default|GetSpline) (Math|Conversions|ToFloat(Integer) 0) "World") false false)))))