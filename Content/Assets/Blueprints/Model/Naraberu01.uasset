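; Naraberu01 is a construction-script Blueprint that lines up copies of a mesh along a spline.
; It loops over Count and adds an InstancedStaticMesh instance at evenly spaced distances along the spline's length.
; Each instance takes the spline's local location and rotation at that distance with unit scale, and none lands at the spline's end distance.
; The event graph holds only disabled, empty default events.
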(event EventBeginPlay)

(event Collision|EventActorBeginOverlap
  (params (OtherActor :type Actor%20Object%20Reference)))

(event EventTick
  (params (DeltaSeconds :type Float%20%28single-precision%29)))

(fn ConstructionScript
  (for _index (range 0 (- (Variables|Default|GetCount) 1))
    (Components|InstancedStaticMesh|AddInstance (Variables|Default|GetInstancedStaticMesh) (Math|Transform|MakeTransform (Spline|GetLocationatDistanceAlongSpline (Variables|Default|GetSpline) (* (/ _index (Variables|Default|GetCount)) (Spline|GetSplineLength (Variables|Default|GetSpline))) "Local") (Spline|GetRotationatDistanceAlongSpline (Variables|Default|GetSpline) (* (/ _index (Variables|Default|GetCount)) (Spline|GetSplineLength (Variables|Default|GetSpline))) "Local")) false)))