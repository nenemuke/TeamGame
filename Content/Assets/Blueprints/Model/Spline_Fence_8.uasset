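; Spline fence actor that lays park fence meshes along an editable spline.
; The construction script syncs the spline to the root transform, then adds one spline mesh per segment, attached to the spline.
; Each piece bends the fence mesh along X between neighboring points using their local locations and tangents, with query and physics collision enabled.
; The event graph holds only unused default events.
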(event EventBeginPlay)

(event Collision|EventActorBeginOverlap
  (params (OtherActor :type Actor%20Object%20Reference)))

(event EventTick
  (params (DeltaSeconds :type Float%20%28single-precision%29)))

(fn ConstructionScript
  (bind _spline (Variables|Default|GetSpline))
  ;[1 1 1] Transformの同期
  (Transformation|SetWorldTransform (Variables|Default|GetSpline) (Transformation|GetWorldTransform (Variables|Default|GetDefaultSceneRoot)) false false)
  ;[1 1 1] セグメントの数だけ処理を実行
  (for _index (range 0 (- (Class|SplineComponent|GetNumberOfSplineSegments (Variables|Default|GetSpline)) 1))
    (bind _returnvalue (AddComponent|AddSplineMeshComponent false))
    (Transformation|AttachComponentToComponent _returnvalue (Variables|Default|GetSpline) "None" "KeepRelative" "KeepRelative" "KeepRelative" true)
    (SplineMesh|SetForwardAxis _returnvalue "X" true)
    (Components|StaticMesh|SetStaticMesh _returnvalue "/Game/DownloadAssets/CityPark/Meshes/Props/SM_ParkFence01.SM_ParkFence01")
    (SplineMesh|SetStartandEnd _returnvalue (.Location (Spline|GetLocationandTangentatSplinePoint _spline _index "Local")) (.Tangent (Spline|GetLocationandTangentatSplinePoint _spline _index "Local")) (.Location (Spline|GetLocationandTangentatSplinePoint _spline (+ _index 1) "Local")) (.Tangent (Spline|GetLocationandTangentatSplinePoint _spline (+ _index 1) "Local")) true :!class /Script/Engine.SplineMeshComponent)
    (Collision|SetCollisionEnabled _returnvalue "QueryAndPhysics")))