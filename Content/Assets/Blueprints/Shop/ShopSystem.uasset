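; Shop system Blueprint that currently holds test hooks for changing and checking the player's money.
; Its BeginPlay function casts the passed-in object to MyGameInstance and caches it.
; Test events add or deduct fixed amounts through the game instance's GetMoney, using a negative value to spend, and print the balance stored in its PlayerData.
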(event Custom|TestPrintMoney
  (Development|PrintString 0 (Utilities|String|ToString(Integer) (Variables|/Game/Assets/Blueprints/Save/SavePlayerData.SavePlayerData_C|GetMoney (Variables|/Game/Assets/Blueprints/Save/MyGameInstance.MyGameInstance_C|GetPlayerData (Variables|Default|GetGameInstance))))))

(event Custom|TestGetMoney
  (Default|GetMoney (Variables|Default|GetGameInstance) 1000))

(event Custom|TestUseMoney
  (Default|GetMoney (Variables|Default|GetGameInstance) -300))

(fn BeginPlay
  (params (Object :type Object%20Object%20Reference))
  (bind _asmy_game_instance (Utilities|Casting|CastToMyGameInstance Object))
  (Variables|Default|SetGameInstance _asmy_game_instance))