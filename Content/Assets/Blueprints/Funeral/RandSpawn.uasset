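; Funeral spawner actor that recreates the animals recorded as dead in MyGameInstance.
; On BeginPlay it walks the game instance's death name array and maps the matching class-name entry at each index to an Assist animal class.
; Each animal spawns at a random point inside the Box component, gets skeletal mesh physics simulation enabled so it drops as a physical body, and receives its recorded name.
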(event EventBeginPlay
  (bind _box (Variables|Default|GetBox))
  (bind _asmy_game_instance (Utilities|Casting|CastToMyGameInstance (Game|GetGameInstance)))
  (Variables|Default|SetGameInstance _asmy_game_instance)
  (for (_array_element _array_index) (Variables|/Game/Assets/Blueprints/Save/MyGameInstance.MyGameInstance_C|GetDeathAnimalNameArry _asmy_game_instance)
    (switch string (Utilities|Array|Get(acopy) (Variables|/Game/Assets/Blueprints/Save/MyGameInstance.MyGameInstance_C|GetDeathAnimalClassNameArry _asmy_game_instance) _array_index)
      (:Fox
        (Variables|Default|SetSpawnAnimalClass "/Game/Assets/Blueprints/AssistObj/AssistAnimal/AssistFox.AssistFox_C"))
      (:Crocodile
        (Variables|Default|SetSpawnAnimalClass "/Game/Assets/Blueprints/AssistObj/AssistAnimal/AssistCrocodile.AssistCrocodile_C"))
      (:Crow
        (Variables|Default|SetSpawnAnimalClass "/Game/Assets/Blueprints/AssistObj/AssistAnimal/AssistCrow.AssistCrow_C"))
      (:Elephant
        (Variables|Default|SetSpawnAnimalClass "/Game/Assets/Blueprints/AssistObj/AssistAnimal/AssistElephant.AssistElephant_C"))
      (:DeerStag
        (Variables|Default|SetSpawnAnimalClass "/Game/Assets/Blueprints/AssistObj/AssistAnimal/AssistDeerStag.AssistDeerStag_C"))
      (:Hippopotamus
        (Variables|Default|SetSpawnAnimalClass "/Game/Assets/Blueprints/AssistObj/AssistAnimal/AssistHippopotamus.AssistHippopotamus_C"))
      (:Lion
        (Variables|Default|SetSpawnAnimalClass "/Game/Assets/Blueprints/AssistObj/AssistAnimal/AssistLion.AssistLion_C"))
      (:Pig
        (Variables|Default|SetSpawnAnimalClass "/Game/Assets/Blueprints/AssistObj/AssistAnimal/AssistPig.AssistPig_C"))
      (:Rhinoceros
        (Variables|Default|SetSpawnAnimalClass "/Game/Assets/Blueprints/AssistObj/AssistAnimal/AssistRhinoceros.AssistRhinoceros_C"))
      (:Wolf
        (Variables|Default|SetSpawnAnimalClass "/Game/Assets/Blueprints/AssistObj/AssistAnimal/AssistWolf.AssistWolf_C"))
      (:Zebra
        (Variables|Default|SetSpawnAnimalClass "/Game/Assets/Blueprints/AssistObj/AssistAnimal/AssistZebra.AssistZebra_C")))
    (bind _returnvalue (Game|SpawnActorfromClass (Variables|Default|GetSpawnAnimalClass) (Math|Transform|MakeTransform (Math|Random|RandomPointinBoundingBox (Transformation|GetWorldLocation _box) (Variables|/Script/Engine.BoxComponent|GetBoxExtent _box))) "Undefined" 0 "None" 0))
    (Physics|SetSimulatePhysics (Variables|/Game/Assets/Blueprints/AssistObj/AssistAnimal/AssistAnimalBase.AssistAnimalBase_C|GetSkeletalMesh _returnvalue) true)
    (Default|SetAnimalName _returnvalue (Utilities|String|StringToName _array_element))))

(fn ConstructionScript)