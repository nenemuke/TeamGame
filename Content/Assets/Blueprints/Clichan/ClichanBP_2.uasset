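; Player pawn for Clichan, which takes over AI animals through a "Ketsugo" (fusion) attack on left click.
; After the montage, a camera trace against each animal's KetsugoCollision swaps the hit AI for a playable pawn, carries over name, status and HP, possesses it and destroys Clichan.
; Human AIs targeting that animal are retargeted to the new pawn.
; Tick aligns the Box to the camera and tilts the mesh with WASD; Box overlaps toggle UI.
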(event OnComponentBeginOverlap(Box)
  (params (OverlappedComponent :type Primitive%20Component%20Object%20Reference) (OtherActor :type Actor%20Object%20Reference) (OtherComp :type Primitive%20Component%20Object%20Reference) (OtherBodyIndex :type Integer) (bFromSweep :type Boolean) (SweepResult :type Hit%20Result%20Structure%20%28by%20ref%29))
  (Utilities|Casting|CastToAnimalBP OtherActor)
  (Variables|Default|SetlinkPossible_0 true)
  (UserInterface|Viewport|AddtoViewport (Variables|Default|GetPlayerUI) 0))

(event OnComponentEndOverlap(Box)
  (params (OverlappedComponent :type Primitive%20Component%20Object%20Reference) (OtherActor :type Actor%20Object%20Reference) (OtherComp :type Primitive%20Component%20Object%20Reference) (OtherBodyIndex :type Integer))
  (Utilities|Casting|CastToAnimalBP OtherActor)
  (Variables|Default|SetlinkPossible_0 false)
  (Widget|RemovefromParent (Variables|Default|GetPlayerUI)))

(event EventTick
  (params (DeltaSeconds :type Float%20%28single-precision%29))
  (|CallParentFunction DeltaSeconds)
  (|カメラの方向向く)
  (|体を回転される処理))

(event EventBeginPlay
  (bind _box (Variables|Default|GetBox))
  (bind _returnvalue (Transformation|GetRelativeTransform _box))
  (Variables|Default|SetIsClichan true)
  (Variables|Default|SetStatus (Utilities|Struct|MakeAnimalStatus 1e+02 2e+01 15.0 0.0 0 0.7 8.0 "/Game/AnimalVarietyPack/Fox/Animations/ANIM_Fox_Bite_Montage.ANIM_Fox_Bite_Montage" 6e+02 0.0 6e+02 6e+01 0.0 0.0 0.0 "NewEnumerator0" 0))
  (|CallParentFunction)
  (bind _returnvalue_2 (UserInterface|CreateWidget "/Game/Assets/UI/playerUI.playerUI_C"))
  (Variables|Default|SetPlayerUI _returnvalue_2)
  (Transformation|SetRelativeRotation _box (Math|Rotator|MakeRotator 0.0 (.pitch (.rotation _returnvalue)) (.yaw (.rotation _returnvalue))) false false))

(event Input|MouseEvents|LeftMouseButton
  (params (Key :type Key%20Structure))
  (bind _returnvalue (Game|GetPlayerController 0))
  (bind _camera (Variables|Default|GetCamera))
  (bind _returnvalue_2 (Transformation|GetWorldLocation _camera))
  (:Pressed
    (Animation|Montage|PlayMontage (Variables|Default|GetSkeletalMesh) "/Game/Assets/Models/Characeters/Cli-chan/Cli-chan_Anim_アーマチュア_ANIM_Ketugou_Montage.Cli-chan_Anim_アーマチュア_ANIM_Ketugou_Montage"
      (:then
        (Variables|Default|SetIsPlayKetsugoAnime true)
        (Utilities|FlowControl|Delay 1.0)
        (Utilities|Array|Clear (Variables|Default|GetTargetAI))
        (bind _outactors (Actor|GetAllActorsOfClass "/Game/Assets/Blueprints/Animal/AI/AnimalAIBP.AnimalAIBP_C"))
        (for _array_element _outactors
          (Utilities|Array|Add (Variables|Default|GetKetsugo%20Collision) (Variables|/Game/Assets/Blueprints/Animal/AI/AnimalAIBP.AnimalAIBP_C|GetKetsugoCollision _array_element))
          (bind (_hitlocation _hitnormal _bonename _outhit _returnvalue_3) (Collision|LineTraceComponent (Variables|/Game/Assets/Blueprints/Animal/AI/AnimalAIBP.AnimalAIBP_C|GetKetsugoCollision _array_element) _returnvalue_2 (+ _returnvalue_2 (* (Math|Vector|GetForwardVector (Transformation|GetWorldRotation _camera)) (Variables|Default|GetTaleRange))) false false false))
          (if _returnvalue_3
            (Variables|Default|SetHit%20Actor (.HitActor (Collision|BreakHitResult _outhit)))
            (|ステータス記録)
            (|敵に見つかっていないか確かめる)
            (bind _aspawn (|DestoryAndSpawn))
            (|Targetの指定
              (:Completed
                (Pawn|UnPossess _returnvalue)
                (Pawn|Possess _returnvalue _aspawn)
                (bind _asmy_controller (Utilities|Casting|CastToMyController (Game|GetPlayerController 0)))
                (Default|TargetOff _asmy_controller)
                (|ステータスセット)
                (Actor|DestroyActor)
                (bind _returnvalue_4 (Niagara|SpawnSystemAttached "/Game/Assets/Effects/FXE_Cli-chan_Ketugou_2.FXE_Cli-chan_Ketugou_2" (Variables|Default|GetKetsugo) "None" "0, 0, 0" "0, 0, 0" "KeepRelativeOffset" false))
                (Niagara|SetNiagaraVariable(Vector3) _returnvalue_4 "TargetPosition" (Transformation|GetActorLocation (Variables|Default|GetNextControllPawn))))))))
      (:OnCompleted
        (Variables|Default|SetIsPlayKetsugoAnime false)))))

(fn ConstructionScript)

(fn SpecialAttack)

(event Input|KeyboardEvents|W
  (params (Key :type Key%20Structure))
  (:Pressed
    (Variables|Default|SetIsWKey true))
  (:Released
    (Variables|Default|SetIsWKey false)))

(event Input|KeyboardEvents|A
  (params (Key :type Key%20Structure))
  (:Pressed
    (Variables|Default|SetIsAKey true))
  (:Released
    (Variables|Default|SetIsAKey false)))

(event Input|KeyboardEvents|S
  (params (Key :type Key%20Structure))
  (:Pressed
    (Variables|Default|SetIsSKey true))
  (:Released
    (Variables|Default|SetIsSKey false)))

(event Input|KeyboardEvents|D
  (params (Key :type Key%20Structure))
  (:Pressed
    (Variables|Default|SetIsDKey true))
  (:Released
    (Variables|Default|SetIsDKey false)))