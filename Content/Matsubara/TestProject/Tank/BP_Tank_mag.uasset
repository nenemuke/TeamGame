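; BP_Tank_mag is a tank variant Blueprint that supplies its own stats on top of a parent class.
; BeginPlay fills the Status and NurtureStatus structs, calls the parent, then creates a dynamic material instance on the mesh.
; Tick and Fire are empty, and RotateToTarget only plays a montage with a zero rotation offset.
; Projectile spawning, twin-gun muzzle effects with sound, and the parent Tick call remain as unconnected nodes.
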(event Custom|RotateToTarget
  (Animation|Montage|PlayMontage (Variables|Character|GetMesh) 0
    (:then
      (Transformation|AddLocalRotation (Variables|Character|GetMesh) "0, 0, 0" false false))))

(event Custom|Fire)

(event EventBeginPlay
  (Variables|Default|SetStatus (Utilities|Struct|MakeAnimalAIStatus 1e+02 2e+01 0.0 0.0 0 0.0 0.0 "/Game/FlexibleCombatSystem/Montages/M_Fists_AttackA.M_Fists_AttackA" 0.0 5.0 2e+02 8e+02 1e+02 0.0 0 0.0 0.0))
  (Variables|Default|SetNurtureStatus (Utilities|Struct|MakeNurtureStatus 2e+02 0.0 0.0 0.0 6e+01 0.0 0.0 3.0 5e+01 0.0 1e+01 2e+01 0.0 0.0 3.0 0.0 0.0))
  (|CallParentFunction)
  (Rendering|Material|CreateDynamicMaterialInstance (Variables|Character|GetMesh) 1 0 "None" :!class /Script/Engine.PrimitiveComponent))

(event Collision|EventActorBeginOverlap
  (params (OtherActor :type Actor%20Object%20Reference))
  (|CallParentFunction OtherActor) ; このノードは無効になっているため呼び出せません。\n機能をビルドするにはピンをドラッグしてください。
)

(event EventTick
  (params (DeltaSeconds :type Float%20%28single-precision%29)))

(fn ConstructionScript
  (|CallParentFunction))