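; Human enemy Blueprint, a child variant (mag) that supplies its own stats and a gun firing effect.
; BeginPlay fills the Status struct before calling the parent BeginPlay.
; The Fire event plays a montage on the mesh, then spawns an emitter and sound at the weapon's MuzzleFlash socket.
; Fire is purely presentational here, with no trace, projectile or damage logic.
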(event Custom|Fire
  (bind _weapon (Variables|Default|GetWeapon))
  (bind _returnvalue (Transformation|GetSocketTransform _weapon "MuzzleFlash" "RTS_World"))
  (Animation|Montage|PlayMontage (Variables|Character|GetMesh) 0
    (:then
      (Effects|SpawnEmitteratLocation 0 (.location _returnvalue) (.rotation _returnvalue))
      (Audio|PlaySoundatLocation 0 (.location _returnvalue) "0, 0, 0" 1.0 1.0 0.0 0 0 0 0))))

(event EventBeginPlay
  (Variables|Default|SetStatus (Utilities|Struct|MakeAnimalAIStatus 1e+02 2e+01 0.0 0.0 0 0.0 0.0 "/Game/FlexibleCombatSystem/Montages/M_Fists_AttackA.M_Fists_AttackA" 0.0 5.0 5e+01 8e+02 3.0 1e+01 false 1e+02 2e+01 5e+01 false false 3.0))
  (|CallParentFunction))

(event Collision|EventActorBeginOverlap
  (params (OtherActor :type Actor%20Object%20Reference))
  (|CallParentFunction OtherActor) ; このノードは無効になっているため呼び出せません。\n機能をビルドするにはピンをドラッグしてください。
)

(event EventTick
  (params (DeltaSeconds :type Float%20%28single-precision%29))
  (|CallParentFunction DeltaSeconds) ; このノードは無効になっているため呼び出せません。\n機能をビルドするにはピンをドラッグしてください。
)

(fn ConstructionScript
  (|CallParentFunction))