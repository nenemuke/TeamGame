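; AI controller that runs the BTAnimal behavior tree and picks combat targets for AIBP pawns, animals against humans and vice versa.
; Perception sets the target and focus for living enemies, with an obsession delay limiting target switches.
; Tick feeds the Blackboard with touch, bait, target death and randomized stamina, attack and state-change timers.
; The behavior tree's NowState in turn drives stamina drain and attack countdown.
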(event EventBeginPlay
  (|初期設定))

(event EventTick
  (params (DeltaSeconds :type Float%20%28single-precision%29))
  (|ターゲットが死んだかどうか)
  (|ステートが変わったか確かめる)
  (|スタミナ処理 DeltaSeconds)
  (|殴りかかるまでの時間 DeltaSeconds)
  (|時間で他のステートに遷移 DeltaSeconds)
  (|AIが敵に触れたかどうか判定する)
  (|肉を感知する処理)
  (|ターゲット変更可能かどうか))

(fn ConstructionScript)

(fn ResetStamina
  (bind _asaibp (Utilities|Casting|CastToAIBP (Pawn|GetControlledPawn)))
  (Variables|Default|SetNowStamina (+ (Variables|/Game/Assets/Blueprints/Animal/AI/AIBP.AIBP_C|GetStamina _asaibp) (Math|Random|RandomFloatinRange 0.0 (/ (Variables|/Game/Assets/Blueprints/Animal/AI/AIBP.AIBP_C|GetStamina _asaibp) 2.0))))
  (AI|Components|Blackboard|SetValueasBool (Variables|Default|GetBlackboard) (Utilities|Name|MakeLiteralName "IsStaminaFinish") false))

(fn RandomStateTimeReset
  (bind _asaibp (Utilities|Casting|CastToAIBP (Pawn|GetControlledPawn)))
  (Variables|Default|SetRandomStateTime (+ (.randomstatetime (Variables|/Game/Assets/Blueprints/Animal/AI/AIBP.AIBP_C|GetStatus _asaibp)) (Math|Random|RandomFloatinRange 0.0 (/ (.randomstatetime (Variables|/Game/Assets/Blueprints/Animal/AI/AIBP.AIBP_C|GetStatus _asaibp)) 2.0))))
  (AI|Components|Blackboard|SetValueasBool (Variables|Default|GetBlackboard) (Utilities|Name|MakeLiteralName "IsRandomStateChange") false))

(fn AISightReset
  (Class|AIPerceptionComponent|ForgetAll (Variables|Default|GetAIPerception)))

(fn SetTargetActor
  (params (TargetActor :type Actor%20Object%20Reference))
  (Variables|Default|SetTargetActor TargetActor))

(event OnTargetPerceptionUpdated(AIPerception)
  (params (Actor :type Actor%20Object%20Reference) (Stimulus :type AI%20Stimulus%20Structure))
  (bind _asaibp (Utilities|Casting|CastToAIBP (Pawn|GetControlledPawn)))
  (if (Variables|/Game/Assets/Blueprints/Animal/AI/AIBP.AIBP_C|GetIsAnimal _asaibp)
    (bind _ashuman_aibp (Utilities|Casting|CastToHumanAIBP Actor))
    (if (> (Variables|/Game/Assets/Blueprints/Animal/AI/AIBP.AIBP_C|GetHP _ashuman_aibp) 0.0)
      (if (.bSuccessfullySensed (Utilities|Struct|BreakAIStimulus Stimulus)) :!label _label
        (if (.obsession (Variables|/Game/Assets/Blueprints/Animal/AI/AIBP.AIBP_C|GetStatus _asaibp))
          (if (== (AI|Components|Blackboard|GetValueasObject (Variables|Default|GetBlackboard) (Utilities|Name|MakeLiteralName "TargetActor")) 0)
            (AI|Components|Blackboard|SetValueasObject (Variables|Default|GetBlackboard) (Utilities|Name|MakeLiteralName "TargetActor") Actor :!label _label_2)
            (Variables|Default|SetTargetActor Actor)
            (Variables|Default|SetIsSightEnemy true)
            (Variables|Default|SetIsTargetChangable false)
            (Variables|/Script/Engine.Pawn|SetbUseControllerRotationYaw (Pawn|GetControlledPawn) true)
            (AI|SetFocus Actor))
          (elif (Variables|Default|GetIsTargetChangable)
            (if (not (== (AI|Components|Blackboard|GetValueasObject (Variables|Default|GetBlackboard) (Utilities|Name|MakeLiteralName "TargetActor")) Actor))
              (goto _label_2))))
        (else
          (Variables|Default|SetIsSightEnemy false :!label _label_3)))
      (else
        (goto _label_3)))
    (else
      (bind _asanimal_bp (Utilities|Casting|CastToAnimal_BP Actor)
        (:then
          (if (> (Variables|/Game/Assets/Blueprints/Animal/Animal_BP.Animal_BP_C|GetHP _asanimal_bp) 0.0)
            (goto _label)
            (else
              (goto _label_3))))
        (:CastFailed
          (bind _asanimal_aibp (Utilities|Casting|CastToAnimalAIBP Actor))
          (if (> (Variables|/Game/Assets/Blueprints/Animal/AI/AIBP.AIBP_C|GetHP _asanimal_aibp) 0.0)
            (goto _label)
            (else
              (goto _label_3))))))))

(event Custom|スタミナ回復
  (bind _asaibp (Utilities|Casting|CastToAIBP (Pawn|GetControlledPawn)))
  (Variables|Default|SetNowStamina (+ (Variables|/Game/Assets/Blueprints/Animal/AI/AIBP.AIBP_C|GetStamina _asaibp) (Math|Random|RandomFloatinRange 0.0 (/ (Variables|/Game/Assets/Blueprints/Animal/AI/AIBP.AIBP_C|GetStamina _asaibp) 2.0)))))